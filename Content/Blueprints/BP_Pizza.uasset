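; BP_Pizza is an actor that plays a one-shot flipbook animation when the left mouse button is pressed.
; BeginPlay turns looping off on its PaperFlipbook component, and each accepted click plays it from the start.
; Clicks are gated by the Fireable flag, which a click clears and Tick restores once a half-second AnimationCoolDown counts down.
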(event EventBeginPlay
  (Components|Timeline|SetLooping (Variables|Default|GetPaperFlipbook) false))

(event Collision|EventActorBeginOverlap
  (params (OtherActor :type Actor%20Object%20Reference)))

(event EventTick
  (params (DeltaSeconds :type Float%20%28single-precision%29))
  (Variables|Default|SetAnimationCoolDown (- (Variables|Default|GetAnimationCoolDown) DeltaSeconds))
  (if (<= (Variables|Default|GetAnimationCoolDown) 0.0)
    (Variables|Default|SetFireable true)))

(event Input|MouseEvents|LeftMouseButton
  (params (Key :type Key%20Structure :default "None"))
  (:Pressed
    (if (Variables|Default|GetFireable)
      (Components|Timeline|PlayfromStart (Variables|Default|GetPaperFlipbook))
      (Variables|Default|SetAnimationCoolDown 0.5)
      (Variables|Default|SetFireable false))))

(fn ConstructionScript)